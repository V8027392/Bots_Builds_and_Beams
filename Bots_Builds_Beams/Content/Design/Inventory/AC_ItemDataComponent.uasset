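; Item data component that turns its owning actor into an inventory pickup, holding an item ID row and quantity.
; On BeginPlay it sets the owning actor to replicate.
; Interacting adds the item to the interactor's inventory system component and, on success, refreshes that inventory and destroys the pickup actor.
; The LookAt function returns an empty string.
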(event `self.ReceiveBeginPlay`
  (`Actor.SetReplicates` (`self.GetOwner`) true))

(event `/Game/Design/Inventory/BI_Interact.InteractWith`
  (params (Owner :type "/Game/Design/Character/BP_Cosmic_Kid Object Reference"))
  (bind _bpc_inventorysystem (`/Game/Design/Character/BP_Cosmic_Kid.BPC_InventorySystem` Owner))
  (bind (_itemid_datatable _itemid_rowname) (break `DataTableRowHandle` (`self.ItemID`)))
  (`/Engine/EditorBlueprintResources/StandardMacros.IsValid` _bpc_inventorysystem
    (:`Is Valid`
      (bind _success (`/Game/Design/Inventory/BPC_InventorySystem.AddToInventory` _bpc_inventorysystem _itemid_rowname (`self.Quantity`)))
      (if _success
        (`/Game/Design/Character/BP_Cosmic_Kid.Refresh Inventory` Owner)
        (`Actor.K2_DestroyActor` (`self.GetOwner`))))))

(fn `LookAt`
  (returns (Message :type Text))
  (return ""))