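; BP_Storage_Cube is an interactable storage container that opens an inventory screen for the player.
; On BeginPlay it creates a WBP_Storage_Cube widget bound to its own inventory component and caches the reference.
; Interacting casts the first player controller to PC_Survival and has its HUD show that cached container widget.
; Its LookAt function returns an empty string.
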(event `self.ReceiveBeginPlay`
  (bind _returnvalue (`|CreateWidget` "/Game/Design/UI/UserInterface/Storage_Cube/WBP_Storage_Cube.WBP_Storage_Cube_C" null (`self.BPC_InventorySystem`)))
  (set `self.Widget Ref` _returnvalue))

(event `/Game/Design/Inventory/BI_Interact.InteractWith`
  (params (Owner :type "/Game/Design/Character/BP_Cosmic_Kid Object Reference"))
  (bind _aspc_survival (cast `/Game/Design/World_Settings/PC_Survival` (`GameplayStatics.GetPlayerController` 0)))
  (`/Game/Design/UI/UserInterface/Heads-UpDisplay/W_Heads_Up_Display.ShowContainer` (`/Game/Design/World_Settings/PC_Survival.HUD` _aspc_survival) (`self.Widget Ref`)))

(fn `LookAt`
  (returns (Message :type Text))
  (return ""))

(fn `UserConstructionScript`)