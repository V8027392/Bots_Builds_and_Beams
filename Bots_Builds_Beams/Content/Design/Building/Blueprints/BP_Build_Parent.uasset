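; BP_Build_Parent is a base Blueprint for a buildable object that materializes in stages through a dissolve effect.
; BeginPlay applies a dynamic dissolve material to BuildModel, and each BuildYouBitch call increments BuildPercentage to drive its Radius parameter.
; On reaching BuildMax it marks itself Built, enables query and physics collision as WorldDynamic, and clears the overlay material.
; LookAt returns an empty string.
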(event `self.ReceiveBeginPlay`
  (bind _returnvalue (`PrimitiveComponent.CreateDynamicMaterialInstance` (`self.BuildModel`) 0 (`self.Dissolve Material`) "None"))
  (bind _output_get (set `self.Mat Inst` _returnvalue))
  (`PrimitiveComponent.SetMaterial` (`self.BuildModel`) 0 _output_get))

(event `self.ReceiveTick`
  (params (DeltaSeconds :type "Float (single-precision)")))

(event `/Game/Design/Inventory/BI_Interact.Build You Bitch`
  (bind _buildmodel (`self.BuildModel`))
  (if (not (`self.Built?`))
    (bind _output_get (set `self.Build Percentage` (+ 1.0 (`self.Build Percentage`))))
    (if (>= _output_get (`self.Build Max`))
      (set `self.Built?` true)
      (set `self.Build Percentage` (`self.Build Max`))
      (`PrimitiveComponent.SetCollisionEnabled` _buildmodel "QueryAndPhysics")
      (`PrimitiveComponent.SetCollisionObjectType` _buildmodel "ECC_WorldDynamic")
      (`MeshComponent.SetOverlayMaterial` (`self.BuildModel`) null)
      (else
        (`MaterialInstanceDynamic.SetScalarParameterValue` (`self.Mat Inst`) "Radius" _output_get)))))

(fn `LookAt`
  (returns (Message :type Text))
  (return ""))

(fn `UserConstructionScript`)