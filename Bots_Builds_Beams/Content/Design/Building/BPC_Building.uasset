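; Building component for BP_Cosmic_Kid that lets the player preview, rotate, place and remove structures listed in DT_Buildables.
; While in build mode, Tick traces from the camera to move a grid-snapped preview mesh, tinted green or red by placement validity from a box overlap check.
; Placing spawns the Blueprint, deducts inventory requirements and exits; continuous placement does neither of the latter.
; Destruction mode traces and destroys actors tagged Buildable.
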(event `self.ReceiveBeginPlay`
  ;[1 0 0] Event Begin Play
  (bind _asbp_cosmic_kid (cast `/Game/Design/Character/BP_Cosmic_Kid` (`self.GetOwner`)))
  (set `self.Owning Player` _asbp_cosmic_kid)
  (bind _outrownames (`DataTableFunctionLibrary.GetDataTableRowNames` "/Game/Design/Building/DT_Buildables.DT_Buildables"))
  (for _array_element _outrownames
    (bind _returnvalue (`|GetDataTableRow` "/Game/Design/Building/DT_Buildables.DT_Buildables" _array_element)
      (:`then`
        (`KismetArrayLibrary.Array_Add` (`self.Buildables`) _returnvalue)))))

(event `self.ReceiveTick`
  (params (DeltaSeconds :type "Float (single-precision)"))
  ;[1 0 0] Event Tick
  (if (`self.bInBuildMode?`)
    (`self.Preview Loop`)))

(event `EnhancedInput|/Game/Design/Input/IA_Build`
  (params (ActionValue :type Boolean) (ElapsedSeconds :type "Float (double-precision)") (TriggeredSeconds :type "Float (double-precision)") (InputAction :type "InputAction Object Reference" :default "/Game/Design/Input/IA_Build.IA_Build"))
  ;[0.03889 1 0] Enter Build Mode
  (:`Started`
    (if (not (`self.bInBuildMode?`))
      (`/Game/Design/Character/BP_Cosmic_Kid.Display Build Menu` (`self.Owning Player`))
      (else
        (bind _output_get (set `self.bInBuildMode?` false :!label _label))
        (set `self.Destruction Mode` _output_get)
        (`self.Open Mesh Selection`)))))

(event `Stop Build Mode`
  ;[0.03889 1 0] Enter Build Mode
  (goto _label))

(event `Preview Loop`
  (bind _returnvalue (`GameplayStatics.GetPlayerCameraManager` 0))
  (bind _returnvalue_2 (`Actor.K2_GetActorLocation` _returnvalue))
  (bind _returnvalue_3 (+ _returnvalue_2 (* (`Actor.GetActorForwardVector` _returnvalue) 2000.0)))
  ;[0 1 0.9735] Preview Loop
  (bind (_outhit _returnvalue_4) (`KismetSystemLibrary.LineTraceSingle` :`Start` _returnvalue_2 :`End` _returnvalue_3 :`TraceChannel` "TraceTypeQuery1" :`DrawTime` 1.0))
  (`|ExecutionSequence`
    (:`then_0`
      (`/Engine/EditorBlueprintResources/StandardMacros.DoOnce` false :!label _label_2
        (:`Completed`
          (bind _returnvalue_5 (`|AddComponentByClass` (`self.Owning Player`) "/Script/Engine.StaticMeshComponent" false (`self.Build Preview Transform`)))
          (bind _output_get (set `self.Preview Mesh` _returnvalue_5))
          (`StaticMeshComponent.SetStaticMesh` _output_get (`.Mesh_7_E78E78C14BEC5F17B9A9FE9A9A0FD245` (break `/Game/Design/Building/Struct_BuildParts` (`|GetArrayItem` (`self.Buildables`) (`self.Buildable Index`)))))
          (`self.Build Material`
            (:`then`
              _)
            (:`else`
              (bind _returnvalue_6 (`PrimitiveComponent.CreateDynamicMaterialInstance` _output_get 0 "/Game/Art/Build/MI_Placement.MI_Placement" "None"))
              (set `self.Build Material` _returnvalue_6)
              (`self.Colour Based on Placement` _returnvalue_4)))
          (`PrimitiveComponent.SetMaterial` _output_get 0 (`self.Build Material`)))))
    (:`then_1`
      (bind _input_vector1 (`self.Round Up For Grid` (`KismetMathLibrary.SelectVector` (`.Location` (`GameplayStatics.BreakHitResult` _outhit)) _returnvalue_3 _returnvalue_4) 25))
      (bind _output_get_2 (set `self.Build Preview Transform` (`KismetMathLibrary.MakeTransform` _input_vector1 (`self.Build Preview Rotation`))))
      (bind _preview_mesh (`self.Preview Mesh`)
        (:`then`
          (`SceneComponent.K2_SetWorldTransform` _preview_mesh _output_get_2 false false)
          (bind _overlapped_ (`self.Check For Overlap`))
          (bind _output_get_3 (set `self.Valid Build?` (== (not _overlapped_) _returnvalue_4)))
          (`self.Colour Based on Placement` _output_get_3))
        (:`else`)))))

(event `Open Mesh Selection`
  ;[0 1 0.9735] Preview Loop
  (bind _preview_mesh (`self.Preview Mesh`)
    (:`then`
      (`StaticMeshComponent.SetStaticMesh` _preview_mesh null))
    (:`else`
      _))
  (set `self.Preview Mesh` null)
  (goto _label_2 :!via `Reset`))

(event `EnhancedInput|/Game/Design/Input/IA_Place_Build`
  (params (ActionValue :type Boolean) (ElapsedSeconds :type "Float (double-precision)") (TriggeredSeconds :type "Float (double-precision)") (InputAction :type "InputAction Object Reference" :default "/Game/Design/Input/IA_Place_Build.IA_Place_Build"))
  (bind ((`Icon_17_8427BB0A49027F6C7B4DC9B81F8FC1EF` _icon) (`Blueprint_10_6121ED73450FD61514929D902969944B` _blueprint) (`Requirements_21_589CEE1A4C19F4CDD0C4A2A957A82FB0` _requirements)) (break `/Game/Design/Building/Struct_BuildParts` (`|GetArrayItem` (`self.Buildables`) (`self.Buildable Index`))))
  ;[0.03889 1 0] Place Build
  (:`Started`
    (if (and (`self.bInBuildMode?`) (`self.Valid Build?`))
      (bind _asbp_cosmic_kid (cast `/Game/Design/Character/BP_Cosmic_Kid` (`self.GetOwner`)))
      (`/Game/Design/Inventory/BPC_InventorySystem.RemoveFromInventory` (`/Game/Design/Character/BP_Cosmic_Kid.BPC_InventorySystem` _asbp_cosmic_kid) _requirements)
      (`|SpawnActorFromClass` _blueprint (`self.Build Preview Transform`) "AlwaysSpawn" "MultiplyWithRoot" null null)
      (`self.Stop Build Mode`))))

(event `EnhancedInput|/Game/Design/Input/IA_Place_Continuous_Build`
  (params (ActionValue :type Boolean) (ElapsedSeconds :type "Float (double-precision)") (TriggeredSeconds :type "Float (double-precision)") (InputAction :type "InputAction Object Reference" :default "/Game/Design/Input/IA_Place_Continuous_Build.IA_Place_Continuous_Build"))
  (:`Started`
    (if (and (`self.bInBuildMode?`) (`self.Valid Build?`))
      (`|SpawnActorFromClass` (`.Blueprint_10_6121ED73450FD61514929D902969944B` (break `/Game/Design/Building/Struct_BuildParts` (`|GetArrayItem` (`self.Buildables`) (`self.Buildable Index`)))) (`self.Build Preview Transform`) "AlwaysSpawn" "MultiplyWithRoot" null null))))

(event `EnhancedInput|/Game/Design/Input/IA_Remove`
  (params (ActionValue :type Boolean) (ElapsedSeconds :type "Float (double-precision)") (TriggeredSeconds :type "Float (double-precision)") (InputAction :type "InputAction Object Reference" :default "/Game/Design/Input/IA_Remove.IA_Remove"))
  (bind _returnvalue (`GameplayStatics.GetPlayerCameraManager` 0))
  (bind _returnvalue_2 (`Actor.K2_GetActorLocation` _returnvalue))
  ;[0.03889 1 0] Remove Placed Build
  (:`Started`
    (if (`self.Destruction Mode`)
      (bind (_outhit _returnvalue_3) (`KismetSystemLibrary.LineTraceSingle` :`Start` _returnvalue_2 :`End` (+ _returnvalue_2 (* (`Actor.GetActorForwardVector` _returnvalue) 700.0)) :`TraceChannel` "TraceTypeQuery1" :`DrawDebugType` "Persistent"))
      (if _returnvalue_3
        (bind (_bblockinghit _binitialoverlap _time _distance _location _impactpoint _normal _impactnormal _physmat _hitactor) (`GameplayStatics.BreakHitResult` _outhit))
        (if (`Actor.ActorHasTag` _hitactor "Buildable")
          (`Actor.K2_DestroyActor` _hitactor))))))

(event `EnhancedInput|/Game/Design/Input/IA_Build_Scroll`
  (params (ActionValue :type "Float (double-precision)") (ElapsedSeconds :type "Float (double-precision)") (TriggeredSeconds :type "Float (double-precision)") (InputAction :type "InputAction Object Reference" :default "/Game/Design/Input/IA_Build_Scroll.IA_Build_Scroll"))
  ;[0.03889 1 0] Scroll Through Buildables
  (:`Started`
    (set `self.Buildable Index` (`KismetMathLibrary.Clamp` (+ (`self.Buildable Index`) ActionValue) 0 (`KismetArrayLibrary.Array_LastIndex` (`self.Buildables`))))
    (`self.Open Mesh Selection`)))

(event `EnhancedInput|/Game/Design/Input/IA_Rotate_Build`
  (params (ActionValue :type Boolean) (ElapsedSeconds :type "Float (double-precision)") (TriggeredSeconds :type "Float (double-precision)") (InputAction :type "InputAction Object Reference" :default "/Game/Design/Input/IA_Rotate_Build.IA_Rotate_Build"))
  (bind (_build_preview_transform_location _build_preview_transform_rotation) (`KismetMathLibrary.BreakTransform` (`self.Build Preview Transform`)))
  ;[0.03889 1 0] Rotate Preview
  (:`Started`
    (set `self.Build Preview Rotation` (`KismetMathLibrary.MakeRotator` (.roll _build_preview_transform_rotation) (.pitch _build_preview_transform_rotation) (+ (.yaw _build_preview_transform_rotation) (select `bool` ActionValue :`false` -5.0 :`true` 5.0 :!type "Float (single-precision)"))))))

(event `Server Build Progress`
  (params (Actor :type "Actor Object Reference"))
  (`/Engine/EditorBlueprintResources/StandardMacros.IsValid` Actor
    (:`Is Valid`
      (message `/Game/Design/Inventory/BI_Interact.Build You Bitch` Actor))))

(fn `Check For Overlap`
  (returns (`Overlapped?` :type Boolean))
  (bind (_origin _boxextent) (`KismetSystemLibrary.GetComponentBounds` (`self.Preview Mesh`)))
  (bind (_outhit _returnvalue) (`KismetSystemLibrary.BoxTraceSingle` _origin _origin (/ _boxextent 1.2) (struct) "TraceTypeQuery1"))
  (return _returnvalue))

(fn `Colour Based on Placement`
  (params (`Hit Surface?` :type Boolean))
  (`MaterialInstanceDynamic.SetVectorParameterValue` (`self.Build Material`) "Colour" (`KismetMathLibrary.SelectColor` (struct :`R` 0.038887 :`G` 1.0 :`A` 1.0) (struct :`R` 1.0 :`A` 1.0) `Hit Surface?`)))

(fn `Round Up For Grid`
  (params (`Input Vector` :type "Vector Structure") (`Round To` :type Integer))
  (returns (`Input Vector1` :type "Vector Structure"))
  (locals (`X Rounded` :type Integer :default 0) (`Y Rounded` :type Integer :default 0))
  (bind _output_get (set `local.X Rounded` (`KismetMathLibrary.Round` (/ (.x `Input Vector`) `Round To`))))
  (bind _output_get_2 (set `local.Y Rounded` (`KismetMathLibrary.Round` (/ (.y `Input Vector`) `Round To`))))
  (return (`KismetMathLibrary.MakeVector` (`KismetMathLibrary.Conv_IntToDouble` (* _output_get `Round To`)) (`KismetMathLibrary.Conv_IntToDouble` (* _output_get_2 `Round To`)) (.z `Input Vector`))))