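; BP_Cosmic_Kid is the player character for a survival game, with Enhanced Input movement, look, jump and a first/third-person camera toggle.
; BeginPlay caches the PC_Survival controller, adds the basic mapping context, then runs the same toggle as the perspective input, flipping the starting perspective.
; Each toggle activates the matching camera, deactivates the other and passes the new perspective to the BPCBuilding component.
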(event `self.ReceiveBeginPlay`
  (bind _perspective (`self.Perspective`))
  (bind _aspc_survival (cast `/Game/Design/World_Settings/PC_Survival` (`self.GetController`)))
  (bind _output_get (set `self.Main Player Controller` _aspc_survival))
  (bind _returnvalue (pcsubsystem `EnhancedInputLocalPlayerSubsystem` _output_get))
  (`/Engine/EditorBlueprintResources/StandardMacros.IsValid` _returnvalue
    (:`Is Valid`
      (`EnhancedInputSubsystemInterface.AddMappingContext` _returnvalue "/Game/Design/Input/IMC_Basic.IMC_Basic" 0 (struct))
      (if (`|EnumEquality` (`self.Perspective`) "NewEnumerator0") :!label _label
        (set `self.Perspective` "NewEnumerator1")
        (else
          (set `self.Perspective` "NewEnumerator0")))
      (`ActorComponent.SetActive` (select `/Game/Design/Character/Enum_Perspective` _perspective :`NewEnumerator0` (`self.ThirdPersonCam`) :`NewEnumerator1` (`self.FirstPersonCam`)) true false)
      (`ActorComponent.SetActive` (select `/Game/Design/Character/Enum_Perspective` _perspective :`NewEnumerator0` (`self.FirstPersonCam`) :`NewEnumerator1` (`self.ThirdPersonCam`)) false false)
      (`/Game/Design/Character/BPC_Building.Update Cam` (`self.BPC_Building`) (`self.Perspective`)))))

(event `EnhancedInput|/Game/Design/Input/IA_Perspective`
  (params (ActionValue :type Boolean) (ElapsedSeconds :type "Float (double-precision)") (TriggeredSeconds :type "Float (double-precision)") (InputAction :type "InputAction Object Reference" :default "/Game/Design/Input/IA_Perspective.IA_Perspective"))
  (:`Started`
    (goto _label)))

(event `EnhancedInput|/Game/Design/Input/IA_Look`
  (params (ActionValue :type "Vector2D Structure") (ElapsedSeconds :type "Float (double-precision)") (TriggeredSeconds :type "Float (double-precision)") (InputAction :type "InputAction Object Reference" :default "/Game/Design/Input/IA_Look.IA_Look"))
  (:`Triggered`
    (`self.AddControllerYawInput` ActionValue_X)
    (`self.AddControllerPitchInput` ActionValue_Y)))

(event `EnhancedInput|/Game/Design/Input/IA_Move`
  (params (ActionValue :type "Vector2D Structure") (ElapsedSeconds :type "Float (double-precision)") (TriggeredSeconds :type "Float (double-precision)") (InputAction :type "InputAction Object Reference" :default "/Game/Design/Input/IA_Move.IA_Move"))
  (:`Triggered`
    (`self.AddMovementInput` (`self.GetActorRightVector`) ActionValue_X)
    (`self.AddMovementInput` (`self.GetActorForwardVector`) ActionValue_Y)))

(event `EnhancedInput|/Game/Design/Input/IA_Jump`
  (params (ActionValue :type Boolean) (ElapsedSeconds :type "Float (double-precision)") (TriggeredSeconds :type "Float (double-precision)") (InputAction :type "InputAction Object Reference" :default "/Game/Design/Input/IA_Jump.IA_Jump"))
  (:`Triggered`
    (`self.Jump`))
  (:`Completed`
    (`self.StopJumping`)))

(fn `UserConstructionScript`)